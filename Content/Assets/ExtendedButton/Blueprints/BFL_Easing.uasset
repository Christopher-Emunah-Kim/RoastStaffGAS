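; Blueprint function library of easing curves that remap a float alpha, from sine, polynomial, exponential and circular shapes to back and bounce.
; Each family has In, Out and InOut functions in closed-form math, with bounce In and InOut built on the piecewise BounceOut.
; Ease clamps alpha to 0–1 and dispatches by CurveType and EaseType, including a Linear passthrough.
; Its Bounce InOut case returns zero instead of calling EaseBounceInOut.
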(fn EaseSinein
  (params (Alpha :type Float%20%28double-precision%29))
  (return (+ (* (Math|Trig|Cos(Radians) (* Alpha (/ (Math|Float|MultiplybyPi 1.0) 2.0))) -1.0) 1.0)))

(fn EaseSineOut
  (params (Alpha :type Float%20%28double-precision%29))
  (return (Math|Trig|Sin(Radians) (* Alpha (/ (Math|Float|MultiplybyPi 1.0) 2.0)))))

(fn EaseSineinOut
  (params (Alpha :type Float%20%28double-precision%29))
  (return (* -0.5 (- (Math|Trig|Cos(Radians) (* Alpha (Math|Float|MultiplybyPi 1.0))) 1.0))))

(fn EaseQuadraticin
  (params (Alpha :type Float%20%28double-precision%29))
  (return (* Alpha Alpha)))

(fn EaseQuadraticOut
  (params (Alpha :type Float%20%28double-precision%29))
  (return (* -1.0 Alpha (- Alpha 2.0))))

(fn EaseQuadraticinOut
  (params (Alpha :type Float%20%28double-precision%29))
  (if (< Alpha 0.5)
    (LocalVariables|SetOutValue (* 2.0 Alpha Alpha))
    (else
      (LocalVariables|SetOutValue (+ (* -2.0 Alpha Alpha) (* 4.0 Alpha) -1.0))))
  (return (LocalVariables|GetOutValue)))

(fn EaseCubicin
  (params (alpha :type Float%20%28double-precision%29))
  (return (* alpha alpha alpha)))

(fn EaseCubicOut
  (params (Alpha :type Float%20%28double-precision%29))
  (LocalVariables|SetF (- Alpha 1.0))
  (return (+ (* (LocalVariables|GetF) (LocalVariables|GetF) (LocalVariables|GetF)) 1.0)))

(fn EaseCubicinOut
  (params (Alpha :type Float%20%28double-precision%29))
  (if (< Alpha 0.5)
    (LocalVariables|SetCubicInOutVal (* 4.0 Alpha Alpha Alpha))
    (else
      (LocalVariables|SetCIO_F (- (* 2.0 Alpha) 2.0))
      (LocalVariables|SetCubicInOutVal (+ (* 0.5 (LocalVariables|GetCIO_F) (LocalVariables|GetCIO_F) (LocalVariables|GetCIO_F)) 1.0))))
  (return (LocalVariables|GetCubicInOutVal)))

(fn EaseQuarticin
  (params (Alpha :type Float%20%28double-precision%29))
  (return (* Alpha Alpha Alpha Alpha)))

(fn EaseQuarticOut
  (params (Alpha :type Float%20%28double-precision%29))
  (LocalVariables|SetQO_F (- Alpha 1.0))
  (return (+ (* (LocalVariables|GetQO_F) (LocalVariables|GetQO_F) (LocalVariables|GetQO_F) (- 1.0 Alpha)) 1.0)))

(fn EaseQuarticinOut
  (params (Alpha :type Float%20%28double-precision%29))
  (if (< Alpha 0.5)
    (LocalVariables|SetQIO_OutVal (* 8.0 Alpha Alpha Alpha Alpha))
    (else
      (LocalVariables|SetQIO_F (- 1.0 Alpha))
      (LocalVariables|SetQIO_OutVal (+ (* -8.0 (LocalVariables|GetQIO_F) (LocalVariables|GetQIO_F) (LocalVariables|GetQIO_F) (LocalVariables|GetQIO_F)) 1.0))))
  (return (LocalVariables|GetQIO_OutVal)))

(fn EaseQuinticin
  (params (Alpha :type Float%20%28double-precision%29))
  (return (* Alpha Alpha Alpha Alpha Alpha)))

(fn EaseQuinticOut
  (params (Alpha :type Float%20%28double-precision%29))
  (LocalVariables|SetQuO_F (- Alpha 1.0))
  (return (+ (* (LocalVariables|GetQuO_F) (LocalVariables|GetQuO_F) (LocalVariables|GetQuO_F) (LocalVariables|GetQuO_F) (LocalVariables|GetQuO_F)) 1.0)))

(fn EaseQuinticinOut
  (params (Alpha :type Float%20%28double-precision%29))
  (if (< Alpha 0.5)
    (LocalVariables|SetQuIO_OutVal (* 16.0 Alpha Alpha Alpha Alpha Alpha))
    (else
      (LocalVariables|SetQuIO_F (- (* Alpha 2.0) 2.0))
      (LocalVariables|SetQuIO_OutVal (+ (* 0.5 (LocalVariables|GetQuIO_F) (LocalVariables|GetQuIO_F) (LocalVariables|GetQuIO_F) (LocalVariables|GetQuIO_F) (LocalVariables|GetQuIO_F)) 1.0))))
  (return (LocalVariables|GetQuIO_OutVal)))

(fn EaseExponentialin
  (params (Alpha :type Float%20%28double-precision%29))
  (return (Math|Float|Power 2.0 (* (- Alpha 1.0) 1e+01))))

(fn EaseExponentialOut
  (params (Alpha :type Float%20%28double-precision%29))
  (return (+ (* (Math|Float|Power 2.0 (* -1e+01 Alpha)) -1.0) 1.0)))

(fn EaseExponentialinOut
  (params (Alpha :type Float%20%28double-precision%29))
  (LocalVariables|SetEIO_T (* Alpha 2.0))
  (if (< (LocalVariables|GetEIO_T) 1.0)
    (LocalVariables|SetEIO_Outval (* 0.5 (Math|Float|Power 2.0 (* 1e+01 (- (LocalVariables|GetEIO_T) 1.0)))))
    (else
      (LocalVariables|SetEIO_T (- (LocalVariables|GetEIO_T) 1.0))
      (LocalVariables|SetEIO_Outval (* 0.5 (+ (* (Math|Float|Power 2.0 (* -1e+01 (LocalVariables|GetEIO_T))) -1.0) 2.0)))))
  (return (LocalVariables|GetEIO_Outval)))

(fn EaseCircularin
  (params (Alpha :type Float%20%28double-precision%29))
  (return (* -1.0 (- (Math|Float|Sqrt (- 1.0 (* Alpha Alpha))) 1.0))))

(fn EaseCircularOut
  (params (Alpha :type Float%20%28double-precision%29))
  (LocalVariables|SetCO_T (- Alpha 1.0))
  (return (Math|Float|Sqrt (- 1.0 (* (LocalVariables|GetCO_T) (LocalVariables|GetCO_T))))))

(fn EaseCircularinOut
  (params (Alpha :type Float%20%28double-precision%29))
  (LocalVariables|SetCIO_T (* Alpha 2.0))
  (if (< (LocalVariables|GetCIO_T) 1.0)
    (LocalVariables|SetCIO_OutVal (* -0.5 (- (Math|Float|Sqrt (- 1.0 (* (LocalVariables|GetCIO_T) (LocalVariables|GetCIO_T)))) 1.0)))
    (else
      (LocalVariables|SetCIO_T (- (LocalVariables|GetCIO_T) 2.0))
      (LocalVariables|SetCIO_OutVal (* 0.5 (+ (Math|Float|Sqrt (- 1.0 (* (LocalVariables|GetCIO_T) (LocalVariables|GetCIO_T)))) 1.0)))))
  (return (LocalVariables|GetCIO_OutVal)))

(fn EaseBackin
  (params (Alpha :type Float%20%28double-precision%29))
  (return (- (* Alpha Alpha Alpha) (* Alpha (Math|Trig|Sin(Radians) (* Alpha (Math|Float|MultiplybyPi 1.0)))))))

(fn EaseBackOut
  (params (Alpha :type Float%20%28double-precision%29))
  (LocalVariables|SetBO_F (- 1.0 Alpha))
  (return (- 1.0 (- (* (LocalVariables|GetBO_F) (LocalVariables|GetBO_F) (LocalVariables|GetBO_F)) (* (LocalVariables|GetBO_F) (Math|Trig|Sin(Radians) (* (LocalVariables|GetBO_F) (Math|Float|MultiplybyPi 1.0))))))))

(fn EaseBackinOut
  (params (Alpha :type Float%20%28double-precision%29))
  (if (< Alpha 0.5)
    (LocalVariables|SetBIO_F (* 2.0 Alpha))
    (LocalVariables|SetBIO_OutVal (* (- (* (LocalVariables|GetBIO_F) (LocalVariables|GetBIO_F) (LocalVariables|GetBIO_F)) (* (LocalVariables|GetBIO_F) (Math|Trig|Sin(Radians) (* (LocalVariables|GetBIO_F) (Math|Float|MultiplybyPi 1.0))))) 0.5))
    (else
      (LocalVariables|SetBIO_F (- 1.0 (- (* 2.0 Alpha) 1.0)))
      (LocalVariables|SetBIO_OutVal (+ (* 0.5 (- 1.0 (- (* (LocalVariables|GetBIO_F) (LocalVariables|GetBIO_F) (LocalVariables|GetBIO_F)) (* (LocalVariables|GetBIO_F) (Math|Trig|Sin(Radians) (* (LocalVariables|GetBIO_F) (Math|Float|MultiplybyPi 1.0))))))) 0.5))))
  (return (LocalVariables|GetBIO_OutVal)))

(fn EaseBouncein
  (params (Alpha :type Float%20%28double-precision%29))
  (return (- 1.0 (EasingFunctions|EaseBounceOut (- 1.0 Alpha)))))

(fn EaseBounceOut
  (params (Alpha :type Float%20%28double-precision%29))
  (LocalVariables|SetBounceOut_T Alpha)
  (if (< (LocalVariables|GetBounceOut_T) (/ 1.0 2.75))
    (LocalVariables|SetBounceOut_OutVal (* 7.5625 (LocalVariables|GetBounceOut_T) (LocalVariables|GetBounceOut_T)))
    (elif (< (LocalVariables|GetBounceOut_T) (/ 2.0 2.75))
      (LocalVariables|SetBounceOut_T (- (LocalVariables|GetBounceOut_T) (/ 1.5 2.75)))
      (LocalVariables|SetBounceOut_OutVal (+ (* 7.5625 (LocalVariables|GetBounceOut_T) (LocalVariables|GetBounceOut_T)) 0.75))
      (elif (< (LocalVariables|GetBounceOut_T) (/ 2.5 2.75))
        (LocalVariables|SetBounceOut_T (- (LocalVariables|GetBounceOut_T) (/ 2.25 2.75)))
        (LocalVariables|SetBounceOut_OutVal (+ (* 7.5625 (LocalVariables|GetBounceOut_T) (LocalVariables|GetBounceOut_T)) 0.9375))
        (else
          (LocalVariables|SetBounceOut_T (- (LocalVariables|GetBounceOut_T) (/ 2.625 2.75)))
          (LocalVariables|SetBounceOut_OutVal (+ (* 7.5625 (LocalVariables|GetBounceOut_T) (LocalVariables|GetBounceOut_T)) 0.984375))))))
  (return (LocalVariables|GetBounceOut_OutVal)))

(fn EaseBounceinOut
  (params (Alpha :type Float%20%28double-precision%29))
  (if (< Alpha 0.5)
    (LocalVariables|SetBncIO_OutVal (* 0.5 (EasingFunctions|EaseBouncein (* Alpha 2.0))))
    (else
      (LocalVariables|SetBncIO_OutVal (+ (* (EasingFunctions|EaseBounceOut (- (* Alpha 2.0) 1.0)) 0.5) 0.5))))
  (return (LocalVariables|GetBncIO_OutVal)))

(fn Ease
  (params (Alpha :type Float%20%28double-precision%29) (CurveType :type E_CurveType%20Enum :default "NewEnumerator1") (EaseType :type E_EaseType%20Enum :default "NewEnumerator1"))
  (bind _returnvalue (Math|Float|Clamp(Float) Alpha))
  (switch Utilities|FlowControl|Switch|SwitchonE_CurveType CurveType
    (:NewEnumerator1
      (return _returnvalue))
    (:NewEnumerator6
      (switch Utilities|FlowControl|Switch|SwitchonE_EaseType EaseType
        (:NewEnumerator1
          (return (EasingFunctions|EaseSinein _returnvalue)))
        (:NewEnumerator6
          (return (EasingFunctions|EaseSineOut _returnvalue)))
        (:NewEnumerator2
          (return (EasingFunctions|EaseSineinOut _returnvalue)))))
    (:NewEnumerator2
      (switch Utilities|FlowControl|Switch|SwitchonE_EaseType EaseType
        (:NewEnumerator1
          (return (EasingFunctions|EaseQuadraticin _returnvalue)))
        (:NewEnumerator6
          (return (EasingFunctions|EaseQuadraticOut _returnvalue)))
        (:NewEnumerator2
          (return (EasingFunctions|EaseQuadraticinOut _returnvalue)))))
    (:NewEnumerator3
      (switch Utilities|FlowControl|Switch|SwitchonE_EaseType EaseType
        (:NewEnumerator1
          (return (EasingFunctions|EaseCubicin _returnvalue)))
        (:NewEnumerator6
          (return (EasingFunctions|EaseCubicOut _returnvalue)))
        (:NewEnumerator2
          (return (EasingFunctions|EaseCubicinOut _returnvalue)))))
    (:NewEnumerator4
      (switch Utilities|FlowControl|Switch|SwitchonE_EaseType EaseType
        (:NewEnumerator1
          (return (EasingFunctions|EaseQuarticin _returnvalue)))
        (:NewEnumerator6
          (return (EasingFunctions|EaseQuarticOut _returnvalue)))
        (:NewEnumerator2
          (return (EasingFunctions|EaseQuarticinOut _returnvalue)))))
    (:NewEnumerator5
      (switch Utilities|FlowControl|Switch|SwitchonE_EaseType EaseType
        (:NewEnumerator1
          (return (EasingFunctions|EaseQuinticin _returnvalue)))
        (:NewEnumerator6
          (return (EasingFunctions|EaseQuinticOut _returnvalue)))
        (:NewEnumerator2
          (return (EasingFunctions|EaseQuinticinOut _returnvalue)))))
    (:NewEnumerator7
      (switch Utilities|FlowControl|Switch|SwitchonE_EaseType EaseType
        (:NewEnumerator1
          (return (EasingFunctions|EaseExponentialin _returnvalue)))
        (:NewEnumerator6
          (return (EasingFunctions|EaseExponentialOut _returnvalue)))
        (:NewEnumerator2
          (return (EasingFunctions|EaseExponentialinOut _returnvalue)))))
    (:NewEnumerator8
      (switch Utilities|FlowControl|Switch|SwitchonE_EaseType EaseType
        (:NewEnumerator1
          (return (EasingFunctions|EaseCircularin _returnvalue)))
        (:NewEnumerator6
          (return (EasingFunctions|EaseCircularOut _returnvalue)))
        (:NewEnumerator2
          (return (EasingFunctions|EaseCircularinOut _returnvalue)))))
    (:NewEnumerator10
      (switch Utilities|FlowControl|Switch|SwitchonE_EaseType EaseType
        (:NewEnumerator1
          (return (EasingFunctions|EaseBackin _returnvalue)))
        (:NewEnumerator6
          (return (EasingFunctions|EaseBackOut _returnvalue)))
        (:NewEnumerator2
          (return (EasingFunctions|EaseBackinOut _returnvalue)))))
    (:NewEnumerator11
      (switch Utilities|FlowControl|Switch|SwitchonE_EaseType EaseType
        (:NewEnumerator1
          (return (EasingFunctions|EaseBouncein _returnvalue)))
        (:NewEnumerator6
          (return (EasingFunctions|EaseBounceOut _returnvalue)))
        (:NewEnumerator2
          (return 0.0))))))