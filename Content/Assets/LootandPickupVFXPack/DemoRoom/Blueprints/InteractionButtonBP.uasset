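; Demo room interaction button that switches a referenced activatable VFX actor on and off.
; Interact alternates between on and off through a FlipFlop, while trigger volume overlap forces on at entry and off at exit without updating that toggle.
; Each change recolors the button's Niagara effect through its UserColor parameter.
; The construction script sets both the button color and referenced effect to the active state.
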(event OnComponentBeginOverlap(TriggervolumeVFX)
  (params (OverlappedComponent :type Primitive%20Component%20Object%20Reference) (OtherActor :type Actor%20Object%20Reference) (OtherComp :type Primitive%20Component%20Object%20Reference) (OtherBodyIndex :type Integer) (bFromSweep :type Boolean) (SweepResult :type Hit%20Result%20Structure%20%28by%20ref%29))
  (Niagara|SetNiagaraVariable(LinearColor) (Variables|Default|GetNS_Interaction) "UserColor" (Variables|Default|GetInteractionColor))
  (Default|ToggleActivation (Variables|Default|GetActivatableVFXRef) true))

(event OnComponentEndOverlap(TriggervolumeVFX)
  (params (OverlappedComponent :type Primitive%20Component%20Object%20Reference) (OtherActor :type Actor%20Object%20Reference) (OtherComp :type Primitive%20Component%20Object%20Reference) (OtherBodyIndex :type Integer))
  (Niagara|SetNiagaraVariable(LinearColor) (Variables|Default|GetNS_Interaction) "UserColor" (Variables|Default|GetNonInteractionColor))
  (Default|ToggleActivation (Variables|Default|GetActivatableVFXRef) false))

(event EventInteract
  (bind _ns_interaction (Variables|Default|GetNS_Interaction))
  (bind _activatablevfxref (Variables|Default|GetActivatableVFXRef))
  (Utilities|FlowControl|FlipFlop
    (:A
      (Niagara|SetNiagaraVariable(LinearColor) _ns_interaction "UserColor" (Variables|Default|GetInteractionColor))
      (Default|ToggleActivation _activatablevfxref true))
    (:B
      (Niagara|SetNiagaraVariable(LinearColor) _ns_interaction "UserColor" (Variables|Default|GetNonInteractionColor))
      (Default|ToggleActivation _activatablevfxref false))))

(fn ConstructionScript
  (Default|ToggleActivation (Variables|Default|GetActivatableVFXRef) true)
  (Niagara|SetNiagaraVariable(LinearColor) (Variables|Default|GetNS_Interaction) "UserColor" (Variables|Default|GetInteractionColor)))