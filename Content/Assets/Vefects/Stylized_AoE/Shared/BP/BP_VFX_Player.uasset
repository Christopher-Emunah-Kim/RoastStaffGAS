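; BP_VFX_Player is a Blueprint from the Vefects Stylized AoE pack that plays a chosen Niagara effect on a timer.
; The construction script assigns the VFX asset to SpawnedVFX, resetting its override parameters.
; On BeginPlay it waits InitialDelay, then activates the effect with a reset.
; With Loop on, it keeps re-activating at DelaySeconds intervals, repeating InitialDelay before every second activation.
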(event EventBeginPlay
  (bind _delayseconds (Variables|Default|GetDelaySeconds))
  (bind _spawnedvfx (Variables|Default|GetSpawnedVFX))
  (if (Variables|Default|GetLoop)
    (Utilities|FlowControl|Delay (Variables|Default|GetinitialDelay) :!label _label)
    (Components|Activation|Activate _spawnedvfx true)
    (Utilities|FlowControl|Delay _delayseconds)
    (Components|Activation|Activate _spawnedvfx true)
    (Utilities|FlowControl|Delay _delayseconds)
    (goto _label)
    (else
      (Utilities|FlowControl|Delay (Variables|Default|GetinitialDelay))
      (Components|Activation|Activate _spawnedvfx true))))

(fn ConstructionScript
  (Class|NiagaraComponent|SetAsset (Variables|Default|GetSpawnedVFX) (Variables|Default|GetVFX) true))