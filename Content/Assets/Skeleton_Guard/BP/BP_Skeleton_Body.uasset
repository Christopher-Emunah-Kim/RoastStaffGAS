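; BP_Skeleton_Body is a skeleton body assembled from separate mesh components for the skull, jaw, limbs and other bone parts.
; Ten seconds after BeginPlay, it sets a boolean to true and uses it to enable physics simulation on the main mesh and every listed part at once.
; The overlap, Tick and construction script are empty, so the timed switch is its only logic.
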(event EventBeginPlay
  (Utilities|FlowControl|Delay 1e+01)
  (Variables|Default|SetNewVar_1 true)
  (Physics|SetSimulatePhysics (Variables|Character|GetMesh) (Variables|Default|GetNewVar_1)))

(event Collision|EventActorBeginOverlap
  (params (OtherActor :type Actor%20Object%20Reference)))

(event EventTick
  (params (DeltaSeconds :type Float%20%28single-precision%29)))

(fn ConstructionScript)